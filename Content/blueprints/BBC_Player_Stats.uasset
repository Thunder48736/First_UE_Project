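; Player stats component that holds health and stamina for BP_ThirdPersonCharacter and writes changes directly to its HUD widget.
; One tick after BeginPlay it caches the owning character and initializes the HUD.
; Decrease functions return true upon depletion, and raising max stamina also refills it, unlike max health.
; IncreaseHealth clamps to max, but IncreaseStamina's clamp tests CurrentHealth instead of CurrentStamina against MaxStamina.
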(event EventBeginPlay
  (Utilities|FlowControl|DelayUntilNextTick)
  (bind _asbp_third_person_character (Utilities|Casting|CastToBP_ThirdPersonCharacter (Components|GetOwner)))
  (Variables|Default|SetPlayer%20Character%20BP _asbp_third_person_character)
  (Progress|SetPercent (Variables|/Game/UI/WB_HUD.WB_HUD_C|GetStaminaBar (Variables|/Game/ThirdPerson/Blueprints/BP_ThirdPersonCharacter.BP_ThirdPersonCharacter_C|GetHUD%20widget (Variables|Default|GetPlayer%20Character%20BP))) (/ (Variables|Stamina|GetCurrent_Stamina) (Variables|Stamina|GetMax_stamina)))
  (Progress|SetPercent (Variables|/Game/UI/WB_HUD.WB_HUD_C|GetHealthBar (Variables|/Game/ThirdPerson/Blueprints/BP_ThirdPersonCharacter.BP_ThirdPersonCharacter_C|GetHUD%20widget (Variables|Default|GetPlayer%20Character%20BP))) (/ (Variables|Health|GetCurrent_health) (Variables|Health|GetMax_Health)))
  (Rendering|Components|TextRender|SetText (Variables|/Game/UI/WB_HUD.WB_HUD_C|GetHealthText (Variables|/Game/ThirdPerson/Blueprints/BP_ThirdPersonCharacter.BP_ThirdPersonCharacter_C|GetHUD%20widget (Variables|Default|GetPlayer%20Character%20BP))) (Utilities|Text|ToText(Float) (Variables|Health|GetCurrent_health) "HalfToEven")))

(fn DecreaceHealth
  (params (Damage :type Float%20%28double-precision%29))
  (bind _player_character_bp (Variables|Default|GetPlayer%20Character%20BP))
  (bind _hud_widget (Variables|/Game/ThirdPerson/Blueprints/BP_ThirdPersonCharacter.BP_ThirdPersonCharacter_C|GetHUD%20widget _player_character_bp))
  (if (not (<= (Variables|Health|GetCurrent_health) 0.0))
    (bind _output_get (Variables|Health|SetCurrent_health (- (Variables|Health|GetCurrent_health) Damage)))
    (Progress|SetPercent (Variables|/Game/UI/WB_HUD.WB_HUD_C|GetHealthBar _hud_widget) (/ _output_get (Variables|Health|GetMax_Health)))
    (Rendering|Components|TextRender|SetText (Variables|/Game/UI/WB_HUD.WB_HUD_C|GetHealthText _hud_widget) (Utilities|Text|ToText(Float) (Variables|Health|GetCurrent_health) "HalfToEven"))
    (if (<= (Variables|Health|GetCurrent_health) 0.0)
      _
      (else
        (return false))))
  (return true))

(fn IncreaseMaxHealth
  (params (Incremation :type Float%20%28double-precision%29))
  (bind _player_character_bp (Variables|Default|GetPlayer%20Character%20BP))
  (bind _hud_widget (Variables|/Game/ThirdPerson/Blueprints/BP_ThirdPersonCharacter.BP_ThirdPersonCharacter_C|GetHUD%20widget _player_character_bp))
  (Variables|Health|SetMax_Health (+ (Variables|Health|GetMax_Health) Incremation))
  (Progress|SetPercent (Variables|/Game/UI/WB_HUD.WB_HUD_C|GetHealthBar _hud_widget) (/ (Variables|Health|GetCurrent_health) (Variables|Health|GetMax_Health)))
  (Rendering|Components|TextRender|SetText (Variables|/Game/UI/WB_HUD.WB_HUD_C|GetHealthText _hud_widget) (Utilities|Text|ToText(Float) (Variables|Health|GetCurrent_health) "HalfToEven")))

(fn DecreaseStamina
  (params (Stamina%20deplited :type Float%20%28double-precision%29))
  (bind _player_character_bp (Variables|Default|GetPlayer%20Character%20BP))
  (bind _hud_widget (Variables|/Game/ThirdPerson/Blueprints/BP_ThirdPersonCharacter.BP_ThirdPersonCharacter_C|GetHUD%20widget _player_character_bp))
  (if (not (<= (Variables|Stamina|GetCurrent_Stamina) 0.0))
    (Variables|Stamina|SetCurrent_Stamina (- (Variables|Stamina|GetCurrent_Stamina) Stamina%20deplited))
    (Progress|SetPercent (Variables|/Game/UI/WB_HUD.WB_HUD_C|GetStaminaBar _hud_widget) (/ (Variables|Stamina|GetCurrent_Stamina) (Variables|Stamina|GetMax_stamina)))
    (Rendering|Components|TextRender|SetText (Variables|/Game/UI/WB_HUD.WB_HUD_C|GetStaminaText _hud_widget) (Utilities|Text|ToText(Float) (Variables|Stamina|GetCurrent_Stamina) "HalfToEven"))
    (if (<= (Variables|Stamina|GetCurrent_Stamina) 0.0)
      _
      (else
        (return false))))
  (return true))

(fn IncreaseMaxStamina
  (params (Added%20stamina :type Float%20%28double-precision%29))
  (bind _player_character_bp (Variables|Default|GetPlayer%20Character%20BP))
  (bind _hud_widget (Variables|/Game/ThirdPerson/Blueprints/BP_ThirdPersonCharacter.BP_ThirdPersonCharacter_C|GetHUD%20widget _player_character_bp))
  (bind _output_get (Variables|Stamina|SetMax_stamina (+ (Variables|Stamina|GetMax_stamina) Added%20stamina)))
  (Variables|Stamina|SetCurrent_Stamina _output_get)
  (Progress|SetPercent (Variables|/Game/UI/WB_HUD.WB_HUD_C|GetStaminaBar _hud_widget) (/ (Variables|Stamina|GetCurrent_Stamina) (Variables|Stamina|GetMax_stamina)))
  (Rendering|Components|TextRender|SetText (Variables|/Game/UI/WB_HUD.WB_HUD_C|GetStaminaText _hud_widget) (Utilities|Text|ToText(Float) (Variables|Stamina|GetCurrent_Stamina) "HalfToEven")))

(fn IncreaseHealth
  (params (Added%20health :type Float%20%28double-precision%29))
  (bind _player_character_bp (Variables|Default|GetPlayer%20Character%20BP))
  (bind _hud_widget (Variables|/Game/ThirdPerson/Blueprints/BP_ThirdPersonCharacter.BP_ThirdPersonCharacter_C|GetHUD%20widget _player_character_bp))
  (Variables|Health|SetCurrent_health (+ (Variables|Health|GetCurrent_health) Added%20health))
  (if (> (Variables|Health|GetCurrent_health) (Variables|Health|GetMax_Health))
    (Variables|Health|SetCurrent_health (Variables|Health|GetMax_Health)))
  (Progress|SetPercent (Variables|/Game/UI/WB_HUD.WB_HUD_C|GetHealthBar _hud_widget) (/ (Variables|Health|GetCurrent_health) (Variables|Health|GetMax_Health)))
  (Rendering|Components|TextRender|SetText (Variables|/Game/UI/WB_HUD.WB_HUD_C|GetHealthText _hud_widget) (Utilities|Text|ToText(Float) (Variables|Health|GetCurrent_health) "HalfToEven")))

(fn IncreaseStamina
  (params (Added%20stamina :type Float%20%28double-precision%29))
  (bind _player_character_bp (Variables|Default|GetPlayer%20Character%20BP))
  (bind _hud_widget (Variables|/Game/ThirdPerson/Blueprints/BP_ThirdPersonCharacter.BP_ThirdPersonCharacter_C|GetHUD%20widget _player_character_bp))
  (Variables|Stamina|SetCurrent_Stamina (+ (Variables|Stamina|GetCurrent_Stamina) Added%20stamina))
  (if (> (Variables|Health|GetCurrent_health) (Variables|Stamina|GetMax_stamina))
    (Variables|Stamina|SetCurrent_Stamina (Variables|Stamina|GetMax_stamina)))
  (Progress|SetPercent (Variables|/Game/UI/WB_HUD.WB_HUD_C|GetStaminaBar _hud_widget) (/ (Variables|Stamina|GetCurrent_Stamina) (Variables|Stamina|GetMax_stamina)))
  (Rendering|Components|TextRender|SetText (Variables|/Game/UI/WB_HUD.WB_HUD_C|GetStaminaText _hud_widget) (Utilities|Text|ToText(Float) (Variables|Stamina|GetCurrent_Stamina) "HalfToEven")))